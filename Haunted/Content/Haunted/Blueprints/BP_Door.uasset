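; BP_Door is a door that toggles open and closed when Dooropen is called, optionally requiring a key.
; If Locked, it checks for KeyNeeded in the KeyRing of the player cast from the Box overlap, otherwise playing a locked sound and printing a hint.
; A FlipFlop alternates playing and reversing a timeline that lerps door yaw through a quarter turn, with open and close sounds.
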(event OnComponentBeginOverlap(Box)
  (params (OverlappedComponent :type Primitive%20Component%20Object%20Reference) (OtherActor :type Actor%20Object%20Reference) (OtherComp :type Primitive%20Component%20Object%20Reference) (OtherBodyIndex :type Integer) (bFromSweep :type Boolean) (SweepResult :type Hit%20Result%20Structure%20%28by%20ref%29))
  (bind _asbp_player (Utilities|Casting|CastToBP_Player OtherActor)
    (:CastFailed
      (Development|PrintString "failed"))))

(event Custom|Door%20open
  (if (Variables|Default|Getlocked?)
    (if (Utilities|Array|ContainsItem (Variables|/Game/Haunted/Blueprints/BP_Player.BP_Player_C|GetKeyRing (stale OnComponentBeginOverlap(Box) _asbp_player)) (Variables|Default|GetkeyNeeded))
      (Utilities|FlowControl|FlipFlop :!label _label
        (:A
          (CallFunction|OpenDoor)
          (bind _dooropen (Timeline|DoorOpen_TL Play)
            (:Update
              (Transformation|SetRelativeRotation (Variables|Default|GetDoor) (Math|Rotator|MakeRotator 0.0 0.0 (Math|Float|Lerp 0.0 9e+01 _dooropen)) false false))))
        (:B
          (CallFunction|CloseDoor)
          (Timeline|DoorOpen_TL Reverse)))
      (else
        (CallFunction|LockedDoor)
        (Development|PrintString "Go find the key!")))
    (else
      (goto _label))))

(fn ConstructionScript)

(fn LockedDoor
  (Audio|PlaySoundatLocation "/Game/Haunted/SoundFX/locked_door.locked_door" (Transformation|GetActorLocation) "0, 0, 0" 1.0 1.0 0.0 0 0 0 0))

(fn OpenDoor
  (Audio|PlaySoundatLocation "/Game/Haunted/SoundFX/open_door.open_door" (Transformation|GetActorLocation) "0, 0, 0" 1.0 1.0 0.0 0 0 0 0))

(fn CloseDoor
  (Audio|PlaySoundatLocation "/Game/Haunted/SoundFX/close_door.close_door" (Transformation|GetActorLocation) "0, 0, 0" 1.0 1.0 0.0 0 0 0 0))