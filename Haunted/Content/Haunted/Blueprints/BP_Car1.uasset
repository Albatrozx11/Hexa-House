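; Drivable car pawn that drives itself forward until its capsule hits a BP_worldCollision, then hands throttle control to the player.
; Steering input turns the controller only while W is held, and the steering wheel's rotation follows the actor's yaw.
; Tick toggles idle and forward components by speed and starts idle or running camera shakes.
; Overlapping BP_Park deactivates CarForward after a delay, and parkwidget briefly shows WB_Park.
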(event OnComponentHit(CapsuleComponent)
  (params (HitComponent :type Primitive%20Component%20Object%20Reference) (OtherActor :type Actor%20Object%20Reference) (OtherComp :type Primitive%20Component%20Object%20Reference) (NormalImpulse :type Vector :default "0, 0, 0") (Hit :type Hit%20Result%20Structure%20%28by%20ref%29))
  ;[1 1 1] Auto Move
  ;;[0.2158 0.7125 1] isPlaying?
  (Utilities|Casting|CastToBP_worldCollision OtherActor)
  (Variables|Default|SetisPlaying? true))

(event Custom|park%20widget
  ;[1 1 1] Parking
  (bind _returnvalue (UserInterface|CreateWidget "/Game/Haunted/Blueprints/WB_Park.WB_Park_C"))
  (UserInterface|Viewport|AddtoViewport _returnvalue 0)
  (Utilities|FlowControl|Delay 3.0)
  (Widget|RemovefromParent _returnvalue))

(event Custom|CameraShakeEvent
  (bind _returnvalue (Game|GetPlayerController 0))
  (if (<= (Math|Vector|VectorLengthXY (Transformation|GetVelocity)) 0.0)
    (Game|Feedback|ClientStartCameraShake _returnvalue "/Game/Haunted/Blueprints/BP_CameraShake_car_idle.BP_CameraShake_car_idle_C" 1.0 "CameraLocal" "0, 0, 0")
    (else
      (Game|Feedback|ClientStartCameraShake _returnvalue "/Game/Haunted/Blueprints/BP_CameraShake_car_running.BP_CameraShake_car_running_C" 1.0 "CameraLocal" "0, 0, 0"))))

(event EventTick
  (params (DeltaSeconds :type Float%20%28single-precision%29))
  (bind _returnvalue (Transformation|GetActorRotation))
  (bind _charactermovement (Variables|Character|GetCharacterMovement))
  (bind _car_idle (Variables|Default|Getcar_idle))
  ;[1 1 1] Auto Move
  (Utilities|FlowControl|Sequence
    (:then_0
      (if (== (Math|Vector|VectorLength (Transformation|GetVelocity)) 0.0)
        (if (Variables|Default|GetisPlaying?)
          (Components|Activation|Activate _car_idle false)
          (else
            (Components|Activation|Deactivate _car_idle :!label _label)))
        (else
          (goto _label))))
    (:then_1
      (Transformation|SetRelativeRotation (Variables|Default|Getsteer_wheel) (Math|Rotator|MakeRotator (.Yaw (Math|Rotator|BreakRotator _returnvalue)) -3e+01 0.0) false false))
    (:then_2
      (if (not (Variables|Default|GetisPlaying?))
        (Pawn|Input|AddMovementInput (Math|Vector|GetForwardVector _returnvalue) (Variables|/Script/Engine.CharacterMovementComponent|GetMaxWalkSpeed _charactermovement) false)
        (if (> (Math|Vector|VectorLength (Variables|/Script/Engine.MovementComponent|GetVelocity _charactermovement)) 0.0)
          (Components|Activation|Activate (Variables|Default|Getcar_forward) false)
          (else
            (Components|Activation|Deactivate (Variables|Default|Getcar_forward))))))
    (:then_3
      (CallFunction|CameraShakeEvent))))

(event Collision|EventActorBeginOverlap
  (params (OtherActor :type Actor%20Object%20Reference))
  ;[1 1 1] Parking
  (bind _asbp_park (Utilities|Casting|CastToBP_Park OtherActor))
  (Utilities|FlowControl|Delay 0.5)
  (Components|Activation|Deactivate (Variables|Default|Getcar_forward)))

(event Input|AxisEvents|InputAxisMoveForward
  (params (AxisValue :type Float%20%28single-precision%29))
  ;[1 1 1] Auto Move
  (if (Variables|Default|GetisPlaying?)
    (Pawn|Input|AddMovementInput (Math|Vector|GetForwardVector (Transformation|GetActorRotation)) AxisValue false)
    (if (> (Math|Vector|VectorLength (Variables|/Script/Engine.MovementComponent|GetVelocity (Variables|Character|GetCharacterMovement))) 0.0)
      (Components|Activation|Activate (Variables|Default|Getcar_forward) false)
      (else
        (Components|Activation|Deactivate (Variables|Default|Getcar_forward))))))

(event Input|AxisEvents|InputAxisMoveRight
  (params (AxisValue :type Float%20%28single-precision%29))
  ;[1 1 1] Camera
  (if (Variables|Default|GetisMovingForward)
    (Pawn|Input|AddControllerYawInput (* AxisValue 0.2))))

(event Input|KeyboardEvents|W
  (params (Key :type Key%20Structure :default "None"))
  ;[1 1 1] Auto Move
  (:Pressed
    (Variables|Default|SetisMovingForward true))
  (:Released
    (Variables|Default|SetisMovingForward false)))

(fn ConstructionScript)